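; BP_simpleComplexDemo is a physics demo actor with icosphere and cube meshes and a plate, apparently for comparing simple and complex collision.
; BeginPlay gathers the five body meshes into an array.
; The Start event runs once, enabling physics simulation on each body and playing the Oscillation timeline.
; That timeline tilts the plate in pitch and half-scaled roll, with yaw held at zero.
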(event EventBeginPlay
  (Variables|Default|SetBodyArray (Utilities|Array|MakeArray (Variables|Default|GetSM_IcoSphere) (Variables|Default|GetSM_IcoSphere2) (Variables|Default|GetSM_IcoSphere1) (Variables|Default|GetSM_Cube_02) (Variables|Default|GetSM_Cube_01))))

(event Collision|EventActorBeginOverlap
  (params (OtherActor :type Actor%20Object%20Reference)))

(event EventTick
  (params (DeltaSeconds :type Float%20%28single-precision%29)))

(event EventStart
  (Utilities|FlowControl|DoOnce false
    (:Completed
      (for _array_element (Variables|Default|GetBodyArray)
        (Physics|SetSimulatePhysics _array_element true)
        (bind (_direction _pitch _roll) (Timeline|Oscillation PlayFromStart)
          (:Update
            (Transformation|SetRelativeRotation (Variables|Default|GetSM_Plate) (Math|Rotator|MakeRotator (/ _roll 2.0) _pitch 0.0) false false)))))))

(fn ConstructionScript)