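; Grenade projectile Blueprint that explodes on a fixed fuse of a few seconds, started by a timer on BeginPlay.
; The explosion event activates the NPSExplosion effect, hides the grenade mesh and spawns a BP_FForce actor at the grenade's location.
; The grenade destroys itself after a short delay.
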(event Custom|explosion
  (Components|Activation|Activate (Variables|Default|GetNPS_Explosion) false)
  (Rendering|SetVisibility (Variables|Default|GetSM_Grenade) false false)
  (Game|SpawnActorfromClass "/Game/Blueprints/BP_FForce.BP_FForce_C" (Math|Conversions|ToTransform(Vector) (Transformation|GetActorLocation)) "Undefined" 0 0)
  (Utilities|FlowControl|Delay 1.0)
  (Actor|DestroyActor))

(event EventBeginPlay
  (Utilities|Time|SetTimerbyEvent (delegate Custom|explosion) 3.0))

(fn ConstructionScript)