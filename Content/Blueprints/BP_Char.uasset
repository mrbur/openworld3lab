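; BP_Char is the player character with movement, look, a gravity gun and a single-use grenade, and it creates the player UI.
; Interact line-traces from the camera and messages actors implementing BPI_Interact.
; The gun traces for simulating components, pulls them in with a timeline, holds them via a PhysicsHandle updated on Tick, and launches them on release.
; Pickup events enable and show each weapon; throwing spawns BP_GrenadeProjectile.
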(event Custom|PickUpGravityGun
  (Rendering|SetVisibility (Variables|Default|GetSK_GravityGun) true false)
  (Variables|Default|SetHasGravityGun true))

(event Custom|Grab
  (bind _camera (Variables|Default|GetCamera))
  (bind _returnvalue (Transformation|GetWorldLocation _camera))
  (bind (_outhit _returnvalue_2) (Collision|LineTraceForObjects _returnvalue (+ _returnvalue (* (Math|Vector|GetForwardVector (Transformation|GetWorldRotation _camera)) 5e+02)) (Variables|Default|GetObject%20Types) false 0 "None" true "(R=1.000000,G=0.000000,B=0.000000,A=1.000000)" "(R=0.000000,G=1.000000,B=0.000000,A=1.000000)" 2.5))
  (if _returnvalue_2
    (if (Physics|IsSimulatingPhysics (.HitComponent (Collision|BreakHitResult _outhit)) "None")
      (Components|Animation|PlayAnimation (Variables|Default|GetSK_GravityGun) "/Game/SkeletalMesh/SK_GravityGun_PickUp.SK_GravityGun_PickUp" false)
      (bind _output_get (Variables|Default|SetGrabComponent (.HitComponent (Collision|BreakHitResult _outhit))))
      (Variables|Default|SetGrabInitialLocation (Transformation|GetWorldLocation _output_get))
      (bind _alpha (Timeline|MoveToGrabPoint PlayFromStart)
        (:Update
          (Transformation|SetWorldLocation (Variables|Default|GetGrabComponent) (Math|Vector|Lerp(Vector) (Variables|Default|GetGrabInitialLocation) (Transformation|GetWorldLocation (Variables|Default|GetGrabLocation)) _alpha) false false))
        (:Finished
          (Variables|Default|SetIsGrabing true)
          (Class|PhysicsHandleComponent|GrabComponentatLocation (Variables|Default|GetPhysicsHandle) (Variables|Default|GetGrabComponent) "None" (Transformation|GetWorldLocation (Variables|Default|GetGrabLocation)))
          (Class|PrimitiveComponent|SetAngularDamping (Variables|Default|GetGrabComponent) 0.9))))))

(event Custom|Drop
  (Components|Animation|PlayAnimation (Variables|Default|GetSK_GravityGun) "/Game/SkeletalMesh/SK_GravityGun_Release.SK_GravityGun_Release" false)
  (Physics|Components|PhysicsHandle|ReleaseComponent (Variables|Default|GetPhysicsHandle))
  (Physics|AddImpulse (Variables|Default|GetGrabComponent) (* (Math|Vector|GetForwardVector (Transformation|GetWorldRotation (Variables|Default|GetCamera))) 1e+04) "None" false)
  (Utilities|FlowControl|Delay 0.5)
  (Variables|Default|SetIsGrabing false))

(event Custom|PickUpGrenade
  (Variables|Default|SetHasGrenade true)
  (Rendering|SetVisibility (Variables|Default|GetSM_Grenade) true false))

(event EventBeginPlay
  (bind _returnvalue (UserInterface|CreateWidget "/Game/Widgets/WI_PlayerUI.WI_PlayerUI_C"))
  (UserInterface|Viewport|AddtoPlayerScreen _returnvalue))

(event Collision|EventActorBeginOverlap
  (params (OtherActor :type Actor%20Object%20Reference)))

(event EventTick
  (params (DeltaSeconds :type Float%20%28single-precision%29))
  (bind _grablocation (Variables|Default|GetGrabLocation))
  (bind _returnvalue (Transformation|GetWorldTransform _grablocation))
  (if (Variables|Default|GetIsGrabing)
    (Class|PhysicsHandleComponent|SetTargetLocationandRotation (Variables|Default|GetPhysicsHandle) (.location _returnvalue) (.rotation _returnvalue))))

(event Input|ActionEvents|InputActionInteract
  (params (Key :type Key%20Structure :default "None"))
  (bind _camera (Variables|Default|GetCamera))
  (bind _returnvalue (Transformation|GetWorldLocation _camera))
  ;[1 1 1] Interact
  (:Pressed
    (bind (_outhit _returnvalue_2) (Collision|LineTraceByChannel _returnvalue (+ _returnvalue (* (Math|Vector|GetForwardVector (Transformation|GetWorldRotation _camera)) 5e+02)) "TraceTypeQuery1" false 0 "None"))
    (if _returnvalue_2
      (if (Utilities|DoesObjectImplementInterface (.HitActor (Collision|BreakHitResult _outhit)) "/Game/Blueprints/BPI_Interact.BPI_Interact_C")
        (Class|BPIInteract|Interaction(Message) (.HitActor (Collision|BreakHitResult _outhit)))))))

(event Input|AxisEvents|InputAxisMoveForward
  (params (AxisValue :type Float%20%28single-precision%29))
  ;[1 1 1] MOVEMENT
  (Pawn|Input|AddMovementInput (Math|Vector|GetForwardVector (Math|Rotator|MakeRotator 0.0 0.0 (.Yaw (Math|Rotator|BreakRotator (Pawn|GetControlRotation :!class /Script/Engine.Pawn))))) AxisValue false))

(event Input|AxisEvents|InputAxisMoveRight
  (params (AxisValue :type Float%20%28single-precision%29))
  ;[1 1 1] MOVEMENT
  (Pawn|Input|AddMovementInput (Math|Vector|GetRightVector (Math|Rotator|MakeRotator 0.0 0.0 (.Yaw (Math|Rotator|BreakRotator (Pawn|GetControlRotation :!class /Script/Engine.Pawn))))) AxisValue false))

(event Input|AxisEvents|InputAxisLookUp
  (params (AxisValue :type Float%20%28single-precision%29))
  ;[1 1 1] MOVEMENT
  (Pawn|Input|AddControllerPitchInput AxisValue))

(event Input|AxisEvents|InputAxisTurn
  (params (AxisValue :type Float%20%28single-precision%29))
  ;[1 1 1] MOVEMENT
  (Pawn|Input|AddControllerYawInput AxisValue))

(event Input|MouseEvents|LeftMouseButton
  (params (Key :type Key%20Structure :default "None"))
  (:Pressed
    (if (Variables|Default|GetHasGravityGun)
      (if (Variables|Default|GetIsGrabing)
        (CallFunction|Drop)
        (else
          (CallFunction|Grab))))))

(event Input|MouseEvents|RightMouseButton
  (params (Key :type Key%20Structure :default "None"))
  (:Pressed
    (if (Variables|Default|GetHasGrenade)
      (Rendering|SetVisibility (Variables|Default|GetSM_Grenade) false false)
      (Game|SpawnActorfromClass "/Game/Blueprints/BP_GrenadeProjectile.BP_GrenadeProjectile_C" (Transformation|GetWorldTransform (Variables|Default|GetGrenadeLocation)) "AdjustIfPossibleButDontSpawnIfColliding" 0 0)
      (Variables|Default|SetHasGrenade false))))

(fn ConstructionScript)