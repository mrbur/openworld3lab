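; BP_HitDetection is a physics demo actor whose lamp lights up when a sphere hits a stop mesh.
; Start enables physics simulation on the icosphere, and a hit on SM_Stop by that sphere switches the lamp on for three seconds, then off.
; The light effect drives an emission parameter on a dynamic material instance of the lamp mesh, created at BeginPlay.
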(event OnComponentHit(SM_Stop)
  (params (HitComponent :type Primitive%20Component%20Object%20Reference) (OtherActor :type Actor%20Object%20Reference) (OtherComp :type Primitive%20Component%20Object%20Reference) (NormalImpulse :type Vector :default "0, 0, 0") (Hit :type Hit%20Result%20Structure%20%28by%20ref%29))
  (if (== OtherComp (Variables|Default|GetSM_IcoSphere))
    (CallFunction|Lighton)
    (Utilities|FlowControl|Delay 3.0)
    (CallFunction|LightOff)))

(event Custom|LightOn
  (Rendering|Material|SetScalarParameterValue (Variables|Default|GetEmission%20MI) "EmissionPower" 2e+01 :!class /Script/Engine.MaterialInstanceDynamic))

(event Custom|LightOff
  (Rendering|Material|SetScalarParameterValue (Variables|Default|GetEmission%20MI) "EmissionPower" 0.0 :!class /Script/Engine.MaterialInstanceDynamic))

(event EventBeginPlay
  (bind _returnvalue (Rendering|Material|CreateDynamicMaterialInstance (Variables|Default|GetSM_Lamp) 0 0 "None" :!class /Script/Engine.PrimitiveComponent))
  (Variables|Default|SetEmission%20MI _returnvalue))

(event Collision|EventActorBeginOverlap
  (params (OtherActor :type Actor%20Object%20Reference)))

(event EventTick
  (params (DeltaSeconds :type Float%20%28single-precision%29)))

(event EventStart
  (Physics|SetSimulatePhysics (Variables|Default|GetSM_IcoSphere) true))

(fn ConstructionScript)